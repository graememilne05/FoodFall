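; Wave-driven spawner that places burger actors at its Sphere component while the player is nearby.
; A looping one-second timer checks distance and the SpawnCap counter on BP_FirstPersonCharacter, incrementing it on each spawn attempt.
; The character's Wave picks the mix: red only early, then yellow, then green, with red's share shrinking.
; Each branch re-rolls its random number, so odds are uneven and some ticks spawn nothing.
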(event Custom|Spawn
  (bind _returnvalue (Math|Random|RandomIntegerinRange 0 3))
  (bind _returnvalue_2 (Math|Random|RandomIntegerinRange 0 5))
  (bind _returnvalue_3 (Math|Random|RandomIntegerinRange 0 5))
  (bind _asbp_first_person_character (Utilities|Casting|CastToBP_FirstPersonCharacter (Game|GetPlayerCharacter 0)))
  (if (< (Transformation|GetDistanceTo _asbp_first_person_character self) 2.5e+03)
    (if (< (Variables|/Game/FirstPerson/Blueprints/BP_FirstPersonCharacter.BP_FirstPersonCharacter_C|GetSpawnCap _asbp_first_person_character) 24)
      (if (>= (Variables|/Game/FirstPerson/Blueprints/BP_FirstPersonCharacter.BP_FirstPersonCharacter_C|GetWave _asbp_first_person_character) 5)
        (if (>= (Variables|/Game/FirstPerson/Blueprints/BP_FirstPersonCharacter.BP_FirstPersonCharacter_C|GetWave _asbp_first_person_character) 7)
          (if (>= (Variables|/Game/FirstPerson/Blueprints/BP_FirstPersonCharacter.BP_FirstPersonCharacter_C|GetWave _asbp_first_person_character) 10)
            (if (== _returnvalue 0)
              (Game|SpawnActorfromClass "/Game/FoodFall/blueprints/enemies/BP_red_burger.BP_red_burger_C" (Transformation|GetWorldTransform (Variables|Default|GetSphere)) "AdjustIfPossibleButDontSpawnIfColliding" "MultiplyWithRoot" 0 0 :!label _label)
              (bind _asbp_first_person_character_2 (Utilities|Casting|CastToBP_FirstPersonCharacter (Game|GetPlayerCharacter 0) :!label _label_2))
              (Variables|/Game/FirstPerson/Blueprints/BP_FirstPersonCharacter.BP_FirstPersonCharacter_C|SetSpawnCap _asbp_first_person_character_2 (+ (Variables|/Game/FirstPerson/Blueprints/BP_FirstPersonCharacter.BP_FirstPersonCharacter_C|GetSpawnCap _asbp_first_person_character_2) 1))
              (elif (== _returnvalue 1)
                (Game|SpawnActorfromClass "/Game/FoodFall/blueprints/enemies/BP_yellow_burger.BP_yellow_burger_C" (Transformation|GetWorldTransform (Variables|Default|GetSphere)) "AdjustIfPossibleButDontSpawnIfColliding" "MultiplyWithRoot" 0 0 :!label _label_3)
                (goto _label_2)
                (elif (== _returnvalue 2)
                  (Game|SpawnActorfromClass "/Game/FoodFall/blueprints/enemies/BP_green_burger.BP_green_burger_C" (Transformation|GetWorldTransform (Variables|Default|GetSphere)) "AdjustIfPossibleButDontSpawnIfColliding" "MultiplyWithRoot" 0 0 :!label _label_4)
                  (goto _label_2)
                  (elif true
                    _))))
            (elif (> _returnvalue_3 1)
              (goto _label)
              (elif (== _returnvalue_3 0)
                (goto _label_3)
                (elif (== _returnvalue_3 1)
                  (goto _label_4)))))
          (elif (!= _returnvalue_2 0)
            (goto _label)
            (elif (== _returnvalue_2 0)
              (goto _label_3))))
        (else
          (goto _label))))))

(event EventBeginPlay
  (Utilities|Time|SetTimerbyEvent (delegate Custom|Spawn) 1.0 true))

(fn ConstructionScript)