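; Saucer enemy that chases the player and awards Chips when killed.
; Tick issues an AI move toward the player, then checks health; death spawns an explosion, destroys the saucer and updates the player's elimination and spawn-cap counters.
; Hitbox overlaps apply damage by projectile class: flying-saucer shots deal less, burger shots deal more and are destroyed.
; Contact damage to the player is unwired, and HitRange does nothing.
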(event OnComponentBeginOverlap(Hitbox)
  (params (OverlappedComponent :type Primitive%20Component%20Object%20Reference) (OtherActor :type Actor%20Object%20Reference) (OtherComp :type Primitive%20Component%20Object%20Reference) (OtherBodyIndex :type Integer) (bFromSweep :type Boolean) (SweepResult :type Hit%20Result%20Structure%20%28by%20ref%29))
  ;[1 1 1] Damage Burger
  (Utilities|Casting|CastToBP_flying_saucer_projectile_pink OtherActor
    (:then
      (Variables|Default|SetSaucer%20Health (- (Variables|Default|GetSaucer%20Health) 45.0) :!label _label))
    (:CastFailed
      (Utilities|Casting|CastToBP_flying_saucer_projectile_green OtherActor
        (:then
          (goto _label))
        (:CastFailed
          (Utilities|Casting|CastToBP_flying_saucer_projectile_blue OtherActor
            (:then
              (goto _label))
            (:CastFailed
              (Utilities|Casting|CastToBP_flying_saucer_projectile_yellow OtherActor
                (:then
                  (goto _label))
                (:CastFailed
                  (bind _asbp_burger_projectile_patty (Utilities|Casting|CastToBP_burger_projectile_patty OtherActor)
                    (:then
                      (Variables|Default|SetSaucer%20Health (- (Variables|Default|GetSaucer%20Health) 1e+02))
                      (Actor|DestroyActor _asbp_burger_projectile_patty))
                    (:CastFailed
                      (bind _asbp_burger_projectile_tomato (Utilities|Casting|CastToBP_burger_projectile_tomato OtherActor)
                        (:then
                          (Variables|Default|SetSaucer%20Health (- (Variables|Default|GetSaucer%20Health) 1e+02))
                          (Actor|DestroyActor _asbp_burger_projectile_tomato))
                        (:CastFailed
                          (bind _asbp_burger_projectile_lettuce (Utilities|Casting|CastToBP_burger_projectile_lettuce OtherActor))
                          (Variables|Default|SetSaucer%20Health (- (Variables|Default|GetSaucer%20Health) 1e+02))
                          (Actor|DestroyActor _asbp_burger_projectile_lettuce))))))))))))))

(event OnComponentBeginOverlap(HitRange)
  (params (OverlappedComponent :type Primitive%20Component%20Object%20Reference) (OtherActor :type Actor%20Object%20Reference) (OtherComp :type Primitive%20Component%20Object%20Reference) (OtherBodyIndex :type Integer) (bFromSweep :type Boolean) (SweepResult :type Hit%20Result%20Structure%20%28by%20ref%29)))

(event EventBeginPlay)

(event EventTick
  (params (DeltaSeconds :type Float%20%28single-precision%29))
  (bind _asbp_first_person_character (Utilities|Casting|CastToBP_FirstPersonCharacter (Game|GetPlayerCharacter 0)))
  (AI|AIMoveTo self (Math|Vector|MakeVector (.x (Transformation|GetActorLocation _asbp_first_person_character)) 6.5e+03 (.z (Transformation|GetActorLocation _asbp_first_person_character))) _asbp_first_person_character 5.0 false
    (:then
      (if (<= (Variables|Default|GetSaucer%20Health) 0.0)
        (Effects|SpawnEmitteratLocation "/Game/Unreal/StarterContent/Particles/P_Explosion.P_Explosion" (Transformation|GetActorLocation))
        (Actor|DestroyActor)
        (Variables|/Game/FirstPerson/Blueprints/BP_FirstPersonCharacter.BP_FirstPersonCharacter_C|SetChips _asbp_first_person_character (+ (Variables|/Game/FirstPerson/Blueprints/BP_FirstPersonCharacter.BP_FirstPersonCharacter_C|GetChips _asbp_first_person_character) 2e+01))
        (Variables|/Game/FirstPerson/Blueprints/BP_FirstPersonCharacter.BP_FirstPersonCharacter_C|SetWaveElims _asbp_first_person_character (+ (Variables|/Game/FirstPerson/Blueprints/BP_FirstPersonCharacter.BP_FirstPersonCharacter_C|GetWaveElims _asbp_first_person_character) 1))
        (Variables|/Game/FirstPerson/Blueprints/BP_FirstPersonCharacter.BP_FirstPersonCharacter_C|SetSpawnCap _asbp_first_person_character (- (Variables|/Game/FirstPerson/Blueprints/BP_FirstPersonCharacter.BP_FirstPersonCharacter_C|GetSpawnCap _asbp_first_person_character) 1))))))

(fn ConstructionScript)