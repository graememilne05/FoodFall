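; Yellow burger enemy that chases the first-person player and damages them on overlap, respecting invincibility frames.
; On BeginPlay it removes itself if too far from the player, freeing spawn cap.
; Tick reissues AIMoveTo and checks health, awarding chips and a wave elimination on death with an explosion.
; Saucer projectiles deal lighter damage, while burger-ingredient projectiles hit harder and are destroyed on impact.
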(event OnComponentBeginOverlap(Hitbox)
  (params (OverlappedComponent :type Primitive%20Component%20Object%20Reference) (OtherActor :type Actor%20Object%20Reference) (OtherComp :type Primitive%20Component%20Object%20Reference) (OtherBodyIndex :type Integer) (bFromSweep :type Boolean) (SweepResult :type Hit%20Result%20Structure%20%28by%20ref%29))
  ;[1 1 1] Damage Burger
  (Utilities|Casting|CastToBP_flying_saucer_projectile_pink OtherActor
    (:then
      (Variables|Default|SetBurger%20Health (- (Variables|Default|GetBurger%20Health) 45.0) :!label _label))
    (:CastFailed
      (Utilities|Casting|CastToBP_flying_saucer_projectile_green OtherActor
        (:then
          (goto _label))
        (:CastFailed
          (Utilities|Casting|CastToBP_flying_saucer_projectile_blue OtherActor
            (:then
              (goto _label))
            (:CastFailed
              (Utilities|Casting|CastToBP_flying_saucer_projectile_yellow OtherActor
                (:then
                  (goto _label))
                (:CastFailed
                  (bind _asbp_burger_projectile_patty (Utilities|Casting|CastToBP_burger_projectile_patty OtherActor)
                    (:then
                      (Variables|Default|SetBurger%20Health (- (Variables|Default|GetBurger%20Health) 1e+02))
                      (Actor|DestroyActor _asbp_burger_projectile_patty))
                    (:CastFailed
                      (bind _asbp_burger_projectile_tomato (Utilities|Casting|CastToBP_burger_projectile_tomato OtherActor)
                        (:then
                          (Variables|Default|SetBurger%20Health (- (Variables|Default|GetBurger%20Health) 1e+02))
                          (Actor|DestroyActor _asbp_burger_projectile_tomato))
                        (:CastFailed
                          (bind _asbp_burger_projectile_lettuce (Utilities|Casting|CastToBP_burger_projectile_lettuce OtherActor))
                          (Variables|Default|SetBurger%20Health (- (Variables|Default|GetBurger%20Health) 1e+02))
                          (Actor|DestroyActor _asbp_burger_projectile_lettuce))))))))))))))

(event Custom|Check%20Distance
  (bind _asbp_first_person_character (Utilities|Casting|CastToBP_FirstPersonCharacter (Game|GetPlayerCharacter 0)))
  (if (>= (Transformation|GetDistanceTo _asbp_first_person_character 0) 3e+03)
    (Variables|/Game/FirstPerson/Blueprints/BP_FirstPersonCharacter.BP_FirstPersonCharacter_C|SetSpawnCap _asbp_first_person_character (- (Variables|/Game/FirstPerson/Blueprints/BP_FirstPersonCharacter.BP_FirstPersonCharacter_C|GetSpawnCap _asbp_first_person_character) 1))
    (Actor|DestroyActor)))

(event Custom|Damage%20Player
  (bind _asbp_first_person_character (Utilities|Casting|CastToBP_FirstPersonCharacter (Game|GetPlayerCharacter 0)))
  (if (Class|PrimitiveComponent|IsOverlappingComponent (Variables|/Game/FirstPerson/Blueprints/BP_FirstPersonCharacter.BP_FirstPersonCharacter_C|GetHitbox _asbp_first_person_character) (Variables|Default|GetHitRange))
    (if (not (> (Variables|/Game/FirstPerson/Blueprints/BP_FirstPersonCharacter.BP_FirstPersonCharacter_C|GetIFrames _asbp_first_person_character) 0.0))
      (Variables|/Game/FirstPerson/Blueprints/BP_FirstPersonCharacter.BP_FirstPersonCharacter_C|SetHealth _asbp_first_person_character (- (Variables|/Game/FirstPerson/Blueprints/BP_FirstPersonCharacter.BP_FirstPersonCharacter_C|GetHealth _asbp_first_person_character) 3e+01))
      (Variables|/Game/FirstPerson/Blueprints/BP_FirstPersonCharacter.BP_FirstPersonCharacter_C|SetIFrames _asbp_first_person_character 45.0))))

(event EventBeginPlay
  (CallFunction|CheckDistance))

(event EventTick
  (params (DeltaSeconds :type Float%20%28single-precision%29))
  (CallFunction|DamagePlayer)
  (bind _asbp_first_person_character (Utilities|Casting|CastToBP_FirstPersonCharacter (Game|GetPlayerCharacter 0)))
  (AI|AIMoveTo self (Transformation|GetActorLocation _asbp_first_person_character) _asbp_first_person_character 5.0 false
    (:then
      (if (<= (Variables|Default|GetBurger%20Health) 0.0)
        (Effects|SpawnEmitteratLocation "/Game/Unreal/StarterContent/Particles/P_Explosion.P_Explosion" (Transformation|GetActorLocation))
        (Variables|/Game/FirstPerson/Blueprints/BP_FirstPersonCharacter.BP_FirstPersonCharacter_C|SetChips _asbp_first_person_character (+ (Variables|/Game/FirstPerson/Blueprints/BP_FirstPersonCharacter.BP_FirstPersonCharacter_C|GetChips _asbp_first_person_character) 2.0))
        (Variables|/Game/FirstPerson/Blueprints/BP_FirstPersonCharacter.BP_FirstPersonCharacter_C|SetWaveElims _asbp_first_person_character (+ (Variables|/Game/FirstPerson/Blueprints/BP_FirstPersonCharacter.BP_FirstPersonCharacter_C|GetWaveElims _asbp_first_person_character) 1))
        (Variables|/Game/FirstPerson/Blueprints/BP_FirstPersonCharacter.BP_FirstPersonCharacter_C|SetSpawnCap _asbp_first_person_character (- (Variables|/Game/FirstPerson/Blueprints/BP_FirstPersonCharacter.BP_FirstPersonCharacter_C|GetSpawnCap _asbp_first_person_character) 1))
        (Actor|DestroyActor)))))

(fn ConstructionScript)