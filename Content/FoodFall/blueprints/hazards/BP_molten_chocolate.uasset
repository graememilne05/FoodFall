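; BP_molten_chocolate is a molten chocolate hazard that drains Health from overlapping first-person characters.
; An end overlap starts a looping timer, whose Damage event subtracts a fixed amount from each BP_FirstPersonCharacter still overlapping on every tick.
; A begin overlap clears that timer only when no character overlaps, so the start and stop triggers appear reversed from the usual pattern.
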(event Custom|Damage
  (for _array_element (Collision|GetOverlappingActors "/Game/FirstPerson/Blueprints/BP_FirstPersonCharacter.BP_FirstPersonCharacter_C" :!class /Script/Engine.Actor)
    (bind _asbp_first_person_character (Utilities|Casting|CastToBP_FirstPersonCharacter _array_element))
    (Variables|/Game/FirstPerson/Blueprints/BP_FirstPersonCharacter.BP_FirstPersonCharacter_C|SetHealth _asbp_first_person_character (- (Variables|/Game/FirstPerson/Blueprints/BP_FirstPersonCharacter.BP_FirstPersonCharacter_C|GetHealth _asbp_first_person_character) 2e+01))))

(event Collision|EventActorEndOverlap
  (params (OtherActor :type Actor%20Object%20Reference))
  (bind _returnvalue (Utilities|Time|SetTimerbyEvent (delegate Custom|Damage) 0.35 true))
  (bind _output_get (Variables|Default|SetTime _returnvalue)))

(event Collision|EventActorBeginOverlap
  (params (OtherActor :type Actor%20Object%20Reference))
  (if (Utilities|Array|IsEmpty (Collision|GetOverlappingActors "/Game/FirstPerson/Blueprints/BP_FirstPersonCharacter.BP_FirstPersonCharacter_C" :!class /Script/Engine.Actor))
    (Utilities|Time|ClearandInvalidateTimerbyHandle (stale Collision|EventActorEndOverlap _output_get))))

(fn ConstructionScript)