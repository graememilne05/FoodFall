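; BP_toaster is a toaster hazard that endlessly launches toast on a fixed cycle from BeginPlay.
; Each cycle spawns two BP_toast actors at the transforms of its two sphere markers and snaps both spring meshes upward.
; After a retriggerable delay the springs drop back by the same offset, and a second delay loops execution back to the spawn.
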(event EventBeginPlay
  (Game|SpawnActorfromClass "/Game/FirstPerson/Blueprints/projectiles/toast/BP_toast.BP_toast_C" (Transformation|GetWorldTransform (Variables|Default|GetSphere)) "Undefined" "OverrideRootScale" 0 0 :!label _label)
  (Game|SpawnActorfromClass "/Game/FirstPerson/Blueprints/projectiles/toast/BP_toast.BP_toast_C" (Transformation|GetWorldTransform (Variables|Default|GetSphere1)) "Undefined" "OverrideRootScale" 0 0)
  (Transformation|AddLocalOffset (Variables|Default|GetSM_toaster_spring_1) "0.000000,0.000000,130.000000" false false)
  (Transformation|AddLocalOffset (Variables|Default|GetSM_toaster_spring_2) "0.000000,0.000000,130.000000" false false)
  (Utilities|FlowControl|RetriggerableDelay 2.5)
  (Transformation|AddLocalOffset (Variables|Default|GetSM_toaster_spring_1) "0.000000,0.000000,-130.000000" false false)
  (Transformation|AddLocalOffset (Variables|Default|GetSM_toaster_spring_2) "0.000000,0.000000,-130.000000" false false)
  (Utilities|FlowControl|RetriggerableDelay 2.5)
  (goto _label))

(fn ConstructionScript)