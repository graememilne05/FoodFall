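; BP_honey is a hazard actor that slows the first-person player character while it overlaps the honey.
; On begin overlap it sets the character's max walk speed to a reduced base scaled by the character's EnergyBoost.
; On end overlap it restores the full base speed with the same multiplier, halving movement inside the honey without storing the previous speed.
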(event Collision|EventActorEndOverlap
  (params (OtherActor :type Actor%20Object%20Reference))
  (bind _asbp_first_person_character (Utilities|Casting|CastToBP_FirstPersonCharacter OtherActor))
  (Variables|/Script/Engine.CharacterMovementComponent|SetMaxWalkSpeed (Variables|/Script/Engine.Character|GetCharacterMovement _asbp_first_person_character) (* (Variables|/Game/FirstPerson/Blueprints/BP_FirstPersonCharacter.BP_FirstPersonCharacter_C|GetEnergyBoost _asbp_first_person_character) 6e+02)))

(event Collision|EventActorBeginOverlap
  (params (OtherActor :type Actor%20Object%20Reference))
  (bind _asbp_first_person_character (Utilities|Casting|CastToBP_FirstPersonCharacter OtherActor))
  (Variables|/Script/Engine.CharacterMovementComponent|SetMaxWalkSpeed (Variables|/Script/Engine.Character|GetCharacterMovement _asbp_first_person_character) (* (Variables|/Game/FirstPerson/Blueprints/BP_FirstPersonCharacter.BP_FirstPersonCharacter_C|GetEnergyBoost _asbp_first_person_character) 3e+02)))

(fn ConstructionScript)