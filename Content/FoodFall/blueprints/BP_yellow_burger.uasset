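; BP_yellow_burger is an enemy burger in FoodFall that chases the first-person player and drains their health.
; Every Tick it reissues AIMoveTo toward the player, then destroys itself if BurgerHealth has run out.
; Overlapping HitRange starts a looping Delay that deals fixed damage each second, with no end-overlap check to stop it.
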(event OnComponentBeginOverlap(HitRange)
  (params (OverlappedComponent :type Primitive%20Component%20Object%20Reference) (OtherActor :type Actor%20Object%20Reference) (OtherComp :type Primitive%20Component%20Object%20Reference) (OtherBodyIndex :type Integer) (bFromSweep :type Boolean) (SweepResult :type Hit%20Result%20Structure%20%28by%20ref%29))
  (bind _asbp_first_person_character (Utilities|Casting|CastToBP_FirstPersonCharacter OtherActor :!label _label))
  (Variables|/Game/FirstPerson/Blueprints/BP_FirstPersonCharacter.BP_FirstPersonCharacter_C|SetHealth _asbp_first_person_character (- (Variables|/Game/FirstPerson/Blueprints/BP_FirstPersonCharacter.BP_FirstPersonCharacter_C|GetHealth _asbp_first_person_character) 25.0))
  (Utilities|FlowControl|Delay 1.0)
  (goto _label))

(event EventBeginPlay)

(event EventTick
  (params (DeltaSeconds :type Float%20%28single-precision%29))
  (bind _asbp_first_person_character (Utilities|Casting|CastToBP_FirstPersonCharacter (Game|GetPlayerCharacter 0)))
  (AI|AIMoveTo self (Transformation|GetActorLocation _asbp_first_person_character) _asbp_first_person_character 5.0 false
    (:then
      (if (<= (Variables|Default|GetBurger%20Health) 0.0)
        (Actor|DestroyActor)))))

(fn ConstructionScript)