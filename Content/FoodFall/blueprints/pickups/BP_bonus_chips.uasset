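; BP_bonus_chips is a pickup that adds a random amount of Chips to the first-person character on overlap.
; A random roll between the character's Cookie value and 50 grants the larger bonus only when it does not exceed Cookie, so higher Cookie values improve those odds.
; It then plays a pickup sound at its location and destroys itself.
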(event Collision|EventActorBeginOverlap
  (params (OtherActor :type Actor%20Object%20Reference))
  ;[1 1 1] Chips Pickup Functionality
  (bind _asbp_first_person_character (Utilities|Casting|CastToBP_FirstPersonCharacter OtherActor))
  (if (<= (Math|Random|RandomIntegerinRange (Variables|/Game/FirstPerson/Blueprints/BP_FirstPersonCharacter.BP_FirstPersonCharacter_C|GetCookie _asbp_first_person_character) 50) (Variables|/Game/FirstPerson/Blueprints/BP_FirstPersonCharacter.BP_FirstPersonCharacter_C|GetCookie _asbp_first_person_character))
    (Variables|/Game/FirstPerson/Blueprints/BP_FirstPersonCharacter.BP_FirstPersonCharacter_C|SetChips _asbp_first_person_character (+ (Variables|/Game/FirstPerson/Blueprints/BP_FirstPersonCharacter.BP_FirstPersonCharacter_C|GetChips _asbp_first_person_character) (Math|Random|RandomIntegerinRange 20 40)))
    (else
      (Variables|/Game/FirstPerson/Blueprints/BP_FirstPersonCharacter.BP_FirstPersonCharacter_C|SetChips _asbp_first_person_character (+ (Variables|/Game/FirstPerson/Blueprints/BP_FirstPersonCharacter.BP_FirstPersonCharacter_C|GetChips _asbp_first_person_character) (Math|Random|RandomIntegerinRange 10 20)))))
  (Audio|PlaySoundatLocation "/Game/FoodFall/sounds/S_pickup.S_pickup" (Transformation|GetActorLocation) "0, 0, 0" 1.0 1.0 0.0 0 0 0 0)
  (Actor|DestroyActor))

(fn ConstructionScript)