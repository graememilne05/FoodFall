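; BP_fridge is an interactable fridge in FoodFall that opens once to release food pickups.
; On Interact, an Opened flag and a DoOnce gate the action, which yaws the top and bottom SceneCapture-named components, apparently the doors, by different angles.
; It then spawns bonus chips and candy corn at fixed world-space offsets from the fridge, adjusting for collisions, and sets Opened.
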(event EventInteract
  ;[1 1 1] Fridge Interaction
  (if (not (Variables|Default|GetOpened))
    (Utilities|FlowControl|DoOnce false
      (:Completed
        (Transformation|AddLocalRotation (Variables|Default|GetSceneCaptureComponentTop) "0.000000,-90.000000,0.000000" false false)
        (Transformation|AddLocalRotation (Variables|Default|GetSceneCaptureComponentBottom) "0.000000,-70.000000,0.000000" false false)
        (Game|SpawnActorfromClass "/Game/FoodFall/blueprints/pickups/BP_bonus_chips.BP_bonus_chips_C" (Math|Transform|MakeTransform (+ (Transformation|GetActorLocation) "-25.000000,150.000000,20.000000")) "AdjustIfPossibleButAlwaysSpawn" "MultiplyWithRoot" 0 0)
        (Game|SpawnActorfromClass "/Game/FoodFall/blueprints/pickups/BP_candy_corn.BP_candy_corn_C" (Math|Transform|MakeTransform (+ (Transformation|GetActorLocation) "-60.000000,75.000000,20.000000")) "AdjustIfPossibleButAlwaysSpawn" "MultiplyWithRoot" 0 0)
        (Variables|Default|SetOpened true)))))

(fn ConstructionScript)